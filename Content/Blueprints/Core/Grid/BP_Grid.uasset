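; BP_Grid is a hexagon grid actor whose tile generation is unfinished.
; Its construction script calls SpawnGrid, which syncs TileSize to HexagonData.MeshSize and teleports the actor to world X/Y zero, keeping its Z.
; Hex spacing math and a nested row/column loop adding HexagonGridShape instances are present but disconnected, so no tiles are spawned.
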(fn `SpawnGrid`
  (locals (Hex_Width :type "Vector Structure") (Hex_Height :type "Vector Structure") (Vertical_Spacing :type "Vector Structure") (Horizontal_Spacing :type "Vector Structure") (x :type "Vector Structure") (y :type "Vector Structure"))
  (bind (_returnvalue_x _returnvalue_y _returnvalue_z) (`KismetMathLibrary.BreakVector` (`self.K2_GetActorLocation`)))
  (`|ExecutionSequence`
    (:`then_0`
      (if (not (== (`/Game/Blueprints/Core/Grid/GridShapes/DataAsset/GridShapeData.MeshSize` (`self.HexagonData`)) (`self.TileSize`)))
        (set `self.TileSize` (`/Game/Blueprints/Core/Grid/GridShapes/DataAsset/GridShapeData.MeshSize` (`self.HexagonData`)))))
    (:`then_1`
      (`self.K2_SetActorLocation` (`KismetMathLibrary.MakeVector` 0.0 0.0 _returnvalue_z) false true))))

(fn `UserConstructionScript`
  (`self.SpawnGrid`))