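; BP_BaseToken is a base token Blueprint placed on a hex tile grid.
; A snap event teleports its scene root to the current hex tile's location, raised by the capsule half height so it rests on the tile.
; Clicking the capsule only prints a placeholder menu message, and an unconnected snap call with a camp vision print never runs.
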(event `self.ReceiveBeginPlay`)

(event `CE_SnapToHexLoc`
  (`SceneComponent.K2_SetWorldLocation` (`self.DefaultSceneRoot`) (+ (`.HexLocation_9_2D11E7E1440147B401A8E49E3E878024` (break `/Game/Blueprints/Hex/STileHexData` (`self.CurrentHexTileData`))) (`KismetMathLibrary.MakeVector` 0.0 0.0 (`CapsuleComponent.CapsuleHalfHeight` (`self.Capsule`)))) false true))

(event `self.Capsule.OnClicked`
  (params (TouchedComponent :type "PrimitiveComponent Object Reference") (ButtonPressed :type "Key Structure"))
  (`KismetSystemLibrary.PrintString` "Display menu "))

(fn `UserConstructionScript`)